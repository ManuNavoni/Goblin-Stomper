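; Player character for Goblin Stomper: an auto-runner that moves along +X, with Enhanced Input jump, mid-air downward stomp and quit.
; Custom events handle coins, energy pickups, launch boosts and death, which reloads the level.
; The Stomp event uses Z velocity cached on Tick: descending hits add energy and bounce the player, otherwise the level restarts.
; At full energy, the stomp input prints "PATADA NUCLEAR" and empties the meter, with unchanged launch force.
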(event `self.ReceiveBeginPlay`
  (bind _asplayer_controller (cast `PlayerController` (`self.GetController`)))
  (`EnhancedInputSubsystemInterface.AddMappingContext` (pcsubsystem `EnhancedInputLocalPlayerSubsystem` _asplayer_controller) "/Game/Inputs/MC_KingHuman.MC_KingHuman" 0 (struct)))

(event `self.ReceiveTick`
  (params (DeltaSeconds :type "Float (single-precision)"))
  (bind (_velocity_x _velocity_y _velocity_z) (`KismetMathLibrary.BreakVector` (`MovementComponent.Velocity` (`self.CharacterMovement`))))
  (`self.AddMovementInput` (5.0 0.0 0.0))
  (bind _output_get (set `self.VelocidadZJugador` _velocity_z)))

(event `EnhancedInput|/Game/Inputs/IA_Saltar`
  (params (ActionValue :type Boolean) (ElapsedSeconds :type "Float (double-precision)") (TriggeredSeconds :type "Float (double-precision)") (InputAction :type "InputAction Object Reference" :default "/Game/Inputs/IA_Saltar.IA_Saltar"))
  (:`Triggered`
    (if (not (`NavMovementComponent.IsFalling` (`self.CharacterMovement`)))
      (`self.Jump`))))

(event `EnhancedInput|/Game/Inputs/IA_Stomp`
  (params (ActionValue :type "Float (double-precision)") (ElapsedSeconds :type "Float (double-precision)") (TriggeredSeconds :type "Float (double-precision)") (InputAction :type "InputAction Object Reference" :default "/Game/Inputs/IA_Stomp.IA_Stomp"))
  (:`Triggered`
    (if (`NavMovementComponent.IsFalling` (`self.CharacterMovement`))
      (if (>= (`self.Energia`) 100)
        ;[1 1 1] Ataque Empoderado
        (`self.LaunchCharacter` (0.0 0.0 -1500.0) false true)
        (`KismetSystemLibrary.PrintString` "PATADA NUCLEAR" true true (struct :`R` 1.0 :`G` 0.058392 :`A` 1.0) 3.0)
        (set `self.Energia` 0)
        (else
          (`self.LaunchCharacter` (0.0 0.0 -1500.0) false true) ; Ataque Normal
        )))))

(event `/Game/Blueprints/BPI_Coleccion.Monedas`
  (bind _output_get (set `self.Monedas_0` (+ (`self.Monedas_0`) 1)))
  (`KismetSystemLibrary.PrintString` (`KismetStringLibrary.Concat_StrStr` "Monedas: \n" (`KismetStringLibrary.Conv_IntToString` _output_get))))

(event `/Game/Blueprints/BPI_Coleccion.Energía`
  (if (< (`self.Energia`) 100)
    (bind _output_get (set `self.Energia` (`KismetMathLibrary.Clamp` (+ (`self.Energia`) 15) 0 100)))
    (`KismetSystemLibrary.PrintString` (`KismetStringLibrary.Concat_StrStr` "Energía: \n" (`KismetStringLibrary.Conv_IntToString` _output_get)))
    (if (== (`self.Energia`) 100)
      (`KismetSystemLibrary.PrintString` "ENERGIZADO" true true (struct :`G` 1.0 :`B` 0.967532 :`A` 1.0) 5.0 :!label _label))
    (else
      (goto _label))))

(event `/Game/Interface/BPI_Stomp.Stomp`
  (if (>= (`self.VelocidadZJugador`) 0.0)
    (`GameplayStatics.OpenLevel` "GoblinStomper_Level1")
    (else
      (bind _output_get (set `self.Energia` (`KismetMathLibrary.Clamp` (+ (`self.Energia`) 10) 0 100)))
      (`KismetSystemLibrary.PrintString` (`KismetStringLibrary.Concat_StrStr` "Energía: \n" (`KismetStringLibrary.Conv_IntToString` _output_get)))
      (if (== (`self.Energia`) 0)
        (`|ExecutionSequence`
          (:`then_0`
            (goto _label))
          (:`then_1`
            _)))
      (`self.LaunchCharacter` (0.0 0.0 1000.0) false true))))

(event `/Game/Interface/BPI_Morir.Morir`
  (`GameplayStatics.OpenLevel` "GoblinStomper_Level1"))

(event `EnhancedInput|/Game/Inputs/IA_QuitGame`
  (params (ActionValue :type Boolean) (ElapsedSeconds :type "Float (double-precision)") (TriggeredSeconds :type "Float (double-precision)") (InputAction :type "InputAction Object Reference" :default "/Game/Inputs/IA_QuitGame.IA_QuitGame"))
  (:`Triggered`
    (`KismetSystemLibrary.QuitGame` null "Quit")))

(event `/Game/Interface/BPI_Launch.Launch`
  (`self.LaunchCharacter` (0.0 0.0 1800.0) false true))

(fn `NewFunction`
  (bind _returnvalue_x (`KismetMathLibrary.BreakVector` (`CharacterMovementComponent.GetCurrentAcceleration` (`self.CharacterMovement`))))
  (`self.AddMovementInput` (1.0 0.0 0.0))
  (`/Engine/EditorBlueprintResources/StandardMacros.CompareFloat` _returnvalue_x
    (:`>`
      (`Controller.SetControlRotation` (`self.GetController`) (`KismetMathLibrary.MakeRotator` 0.0)))
    (:`<`
      (`Controller.SetControlRotation` (`self.GetController`) (`KismetMathLibrary.MakeRotator` 0.0 0.0 180.0)))))

(fn `UserConstructionScript`)